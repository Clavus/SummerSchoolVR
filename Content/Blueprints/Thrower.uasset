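; Thrower blueprint that fires MyProjectile actors from the player's pawn toward the mouse cursor while the left mouse button is held.
; The button opens and closes a Gate on Tick, and a Delay behind it throttles the repeated spawns.
; Each projectile spawns at a fixed world-X offset from the pawn, rotated along the line from the pawn to the cursor's visibility trace hit.
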(event EventTick
  (params (DeltaSeconds :type Float%20%28single-precision%29))
  (bind _returnvalue (Game|GetPlayerController 0))
  (bind _returnvalue_2 (Pawn|GetControlledPawn _returnvalue))
  (bind _returnvalue_3 (Transformation|GetActorLocation _returnvalue_2))
  (Utilities|FlowControl|Gate true
    (:Exit
      (Utilities|FlowControl|Delay 0.2)
      (Game|SpawnActorfromClass "/Game/Blueprints/MyProjectile.MyProjectile_C" (Math|Transform|MakeTransform (+ _returnvalue_3 "100.000000, 0, 0") (Math|Rotator|FindLookatRotation _returnvalue_3 (.Location (Collision|BreakHitResult (.HitResult (Game|Player|GetHitResultUnderCursorbyChannel _returnvalue "TraceTypeQuery1" true)))))) true))))

(event Input|MouseEvents|LeftMouseButton
  (bind _returnvalue (Game|GetPlayerController 0))
  (bind _returnvalue_2 (Pawn|GetControlledPawn _returnvalue))
  (bind _returnvalue_3 (Transformation|GetActorLocation _returnvalue_2))
  (:Pressed
    (Utilities|FlowControl|Gate true) ; enters at Open
  )
  (:Released
    (Utilities|FlowControl|Gate true) ; enters at Close
  ))

(fn ConstructionScript)

(fn NewFunction)