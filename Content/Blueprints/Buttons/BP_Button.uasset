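; BP_Button is a pressure button that actors push by overlapping its trigger, controlling a target Blueprint and Matinee actors.
; Tick checks the list of overlapping actors to play or reverse the Press timeline, with a sound on press.
; The timeline moves the button and fades its dynamic material's emissive glow.
; When it finishes, it toggles the target's message and plays Matinees, reversing them on release only for one trigger method.
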(event OnComponentEndOverlap(Trigger)
  (params (OtherActor :type Actor%20Object%20Reference) (OtherComp :type Primitive%20Component%20Object%20Reference) (OtherBodyIndex :type Integer))
  ;[1 1 1] Handle button overlap events
  (Utilities|Array|RemoveItem (Variables|Default|GetPushing%20Actors) OtherActor))

(event OnComponentBeginOverlap(Trigger)
  (params (OtherActor :type Actor%20Object%20Reference) (OtherComp :type Primitive%20Component%20Object%20Reference) (OtherBodyIndex :type Integer))
  ;[1 1 1] Handle button overlap events
  (Utilities|Array|Add (Variables|Default|GetPushing%20Actors) OtherActor))

(event EventTick
  (params (DeltaSeconds :type Float%20%28single-precision%29))
  (bind _pushing_actors (Variables|Default|GetPushing%20Actors))
  (bind _target_blueprint (Variables|Default|GetTarget%20Blueprint))
  (bind _target_matinee (Variables|Default|GetTarget%20Matinee))
  (bind _returnvalue (Utilities|Array|Length _pushing_actors))
  (bind _returnvalue_2 (== _returnvalue 0))
  ;[1 1 1] Toggle press / reverse
  (if (Variables|Default|GetIs%20being%20pushed)
    (if _returnvalue_2
      (Variables|Default|SetIs%20being%20pushed false)
      (bind (_direction _press _glow) (Timeline|Press Reverse)
        (:Update
          (Transformation|SetRelativeLocation (Variables|BP_Button|GetButton) (Math|Vector|MakeVector 0.0 0.0 _press) false)
          (Rendering|Material|SetVectorParameterValue (Variables|Default|GetButton%20material) "Emissive" (Math|Color|Lerp(LinearColor) :B "(R=0.004986,G=0.046087,B=0.420000,A=1.000000)" :Alpha _glow) :!class /Script/Engine.MaterialInstanceDynamic))
        (:Finished
          (if (Utilities|Enum|Equal(Enum) _direction "Forward")
            ;[1 1 1] Trigger button actions
            (Class|BPIInteractions|Toggle(Message) _target_blueprint true)
            (for _array_element _target_matinee
              (Audio|Components|Audio|Play _array_element))
            (else
              (Class|BPIInteractions|Toggle(Message) _target_blueprint false)
              (if (Utilities|Enum|Equal(Enum) (Variables|Default|GetTrigger%20method) "NewEnumerator1")
                (for _array_element_2 _target_matinee
                  (Utilities|String|Reverse _array_element_2))))))))
    (elif (not _returnvalue_2)
      (Variables|Default|SetIs%20being%20pushed true)
      (Utilities|FlowControl|Sequence
        (:then_0
          (Timeline|Press Play))
        (:then_1
          (Audio|PlaySoundatLocation "/Game/Audio/button24.button24" (Transformation|GetActorLocation)))))))

(fn ConstructionScript
  (bind _returnvalue (Rendering|Material|CreateDynamicMaterialInstance (Variables|BP_Button|GetButton) 0 0 :!class /Script/Engine.PrimitiveComponent))
  (Variables|Default|SetButton%20material _returnvalue))