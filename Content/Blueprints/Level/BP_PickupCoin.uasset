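; BP_PickupCoin is a collectible coin actor that spins every tick and is picked up when the player character overlaps it.
; A DoOnce gate makes pickup fire once: it plays a sound, hides the coin mesh and calls PickUpCoin on MyCharacterExplorationNoHeadBob.
; It then briefly activates a particle burst and destroys itself after a short delay.
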(event EventTick
  (params (DeltaSeconds :type Float%20%28single-precision%29))
  (Transformation|AddRelativeRotation (Variables|Default|GetCoin) "0,2.500000, 0" false))

(event EventActorBeginOverlap
  (params (OtherActor :type Actor%20Object%20Reference))
  (bind _particlesystem (Variables|Default|GetParticleSystem))
  (if (== OtherActor (Game|GetPlayerCharacter 0))
    (Utilities|FlowControl|DoOnce false
      (:Completed
        (Utilities|FlowControl|Sequence
          (:then_0
            (Audio|PlaySoundatLocation "/Game/Audio/mario_coin_sfx.mario_coin_sfx" (Transformation|GetActorLocation)))
          (:then_1
            (Rendering|SetVisibility (Variables|Default|GetCoin) false false))
          (:then_2
            (bind _asmycharacterexplorationnoheadbob_c (Utilities|Casting|CastToMyCharacterExplorationNoHeadBob (Game|GetPlayerCharacter 0)))
            (Default|PickUpCoin _asmycharacterexplorationnoheadbob_c))
          (:then_3
            ;[1 1 1] Play particle system
            (Components|Activation|Activate _particlesystem false)
            (Utilities|FlowControl|Delay 0.2)
            (Components|Activation|Deactivate _particlesystem)
            (Utilities|FlowControl|Delay 2.0)
            (Actor|DestroyActor)))))))

(fn ConstructionScript)