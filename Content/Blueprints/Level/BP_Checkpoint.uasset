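; BP_Checkpoint is a level checkpoint that records itself as the player's respawn point and can teleport the player back to it.
; When the player character first leaves CheckpointBox, a DoOnce sets LastCheckpoint on MyCharacterExplorationNoHeadBob to this actor and prints a confirmation.
; ResetPlayerToCheckpoint moves the player to the SpawnLocation component's world position without sweeping.
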(event OnComponentEndOverlap(CheckpointBox)
  (params (OtherActor :type Actor%20Object%20Reference) (OtherComp :type Primitive%20Component%20Object%20Reference) (OtherBodyIndex :type Integer))
  (bind _returnvalue (Game|GetPlayerCharacter 0))
  (if (== OtherActor _returnvalue)
    ;[1 1 1] Set checkpoint
    (Utilities|FlowControl|DoOnce false
      (:Completed
        (bind _asmycharacterexplorationnoheadbob_c (Utilities|Casting|CastToMyCharacterExplorationNoHeadBob _returnvalue))
        (Development|PrintString "Checkpoint set!")
        (Variables|/Game/Blueprints/MyCharacterExplorationNoHeadBob.MyCharacterExplorationNoHeadBob_C|SetLast%20Checkpoint _asmycharacterexplorationnoheadbob_c self)))))

(fn ConstructionScript)

(fn ResetPlayertoCheckpoint
  (Transformation|SetActorLocation (Game|GetPlayerCharacter 0) (Transformation|GetWorldLocation (Variables|Default|GetSpawnLocation)) false))