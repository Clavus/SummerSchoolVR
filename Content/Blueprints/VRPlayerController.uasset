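; VR player controller that manages HMD settings, gaze interaction, a spawned context menu and a grappling hook.
; HMD settings load from and save to a save slot and apply via console commands.
; Tick adapts screen percentage to frame rate using gates and delays, and turns the pawn or mesh toward the headset.
; A camera trace highlights tagged components through dynamic materials, tracking gaze time; the menu closes when the player walks away.
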(event EventBeginPlay
  ;[1 1 1] Create game save if none exists load game if one does(Allows HMD settings to be saved and loaded)
  (bind _returnvalue (SaveGame|DoesSaveGameExist "HMDSettings"))
  (if _returnvalue
    (bind _returnvalue_2 (SaveGame|LoadGamefromSlot "HMDSettings"))
    (Variables|Default|SetHMDSettingsSave _returnvalue_2)
    (bind _ashmdsettingssave_c (Utilities|Casting|CastToHMDSettingsSave (Variables|Default|GetHMDSettingsSave)))
    (Variables|HMDSettings|SetCurrentSP (Variables|/Game/Blueprints/HMDSettingsSave.HMDSettingsSave_C|GetCurrentSP _ashmdsettingssave_c))
    (Variables|HMDSettings|SetHighestSP (Variables|/Game/Blueprints/HMDSettingsSave.HMDSettingsSave_C|GetHighestSP _ashmdsettingssave_c))
    (Variables|HMDSettings|SetLowestSP (Variables|/Game/Blueprints/HMDSettingsSave.HMDSettingsSave_C|GetLowestSP _ashmdsettingssave_c))
    (Variables|HMDSettings|SetCurrentDistortionScale (Variables|/Game/Blueprints/HMDSettingsSave.HMDSettingsSave_C|GetDistortionScale _ashmdsettingssave_c))
    (else
      (bind _returnvalue_3 (SaveGame|CreateSaveGameObject "/Game/Blueprints/HMDSettingsSave.HMDSettingsSave_C"))
      (Variables|Default|SetHMDSettingsSave _returnvalue_3)
      (bind _ashmdsettingssave_c_2 (Utilities|Casting|CastToHMDSettingsSave (Variables|Default|GetHMDSettingsSave)))
      (Variables|/Game/Blueprints/HMDSettingsSave.HMDSettingsSave_C|SetCurrentSP _ashmdsettingssave_c_2 (Variables|HMDSettings|GetCurrentSP))
      (Variables|/Game/Blueprints/HMDSettingsSave.HMDSettingsSave_C|SetHighestSP _ashmdsettingssave_c_2 (Variables|HMDSettings|GetHighestSP))
      (Variables|/Game/Blueprints/HMDSettingsSave.HMDSettingsSave_C|SetLowestSP _ashmdsettingssave_c_2 (Variables|HMDSettings|GetLowestSP))
      (Variables|/Game/Blueprints/HMDSettingsSave.HMDSettingsSave_C|SetDistortionScale _ashmdsettingssave_c_2 (Variables|HMDSettings|GetCurrentDistortionScale))
      (SaveGame|SaveGametoSlot (Variables|Default|GetHMDSettingsSave) "HMDSettings")))
  (Development|ExecuteConsoleCommand (Utilities|String|Append (Utilities|String|Append (Utilities|String|Append (Utilities|String|Append (Utilities|String|Append "oculusdev on | " "hmdwarp 1=1 | ") "hmdwarp s=") (Utilities|String|ToString(Float) (Variables|HMDSettings|GetCurrentDistortionScale))) " | hmd sp ") (Utilities|String|ToString(Float) (Variables|HMDSettings|GetCurrentSP)))))

(event EventTick
  (params (DeltaSeconds :type Float%20%28single-precision%29))
  (bind _returnvalue (Pawn|GetControlRotation :!class /Script/Engine.Controller))
  (bind _devicerotation (Class|HeadMountedDisplayFunctionLibrary|GetOrientationandPosition))
  (bind _returnvalue_2 (Game|GetPlayerCameraManager 0))
  (bind _highlightedtimechangingobject (Variables|HighlightingAndInteraction|GetHighlightedTimeChangingObject))
  (bind _desiredframerate (Variables|AutoSPVariables|GetDesiredFrameRate))
  (bind _pawnrotationanglekeyhole (Variables|RotatePawnTowardsHMDOrientation|GetPawnRotationAngleKeyhole))
  (bind (_pitch _yaw _roll) (Class|KismetMathLibrary|BreakRot _returnvalue))
  (bind _yaw_2 (Class|KismetMathLibrary|BreakRot _devicerotation))
  (bind _returnvalue_3 (Transformation|GetActorLocation _returnvalue_2))
  (Variables|AutoSPVariables|SetDeltaSeconds DeltaSeconds)
  (Variables|AutoSPVariables|SetCurrentFps (/ 1.0 (Variables|AutoSPVariables|GetDeltaSeconds)))
  (Variables|HMDSettings|SetCurrentSP (Math|Float|Clamp(Float) (Variables|HMDSettings|GetCurrentSP) (Variables|HMDSettings|GetLowestSP) (Variables|HMDSettings|GetHighestSP)))
  (Utilities|FlowControl|Sequence
    (:then_0
      ;[1 1 1] Dynamically change Screen Percentage (SP) if Current FPS is in range of desired fps add to SP if not take from SP only add more SP after 15 seconds
      (if (and (Variables|AutoSPVariables|GetAutoSPEnabled) (Class|HeadMountedDisplayFunctionLibrary|IsHeadMountedDisplayEnabled))
        (Utilities|FlowControl|Delay 2.0)
        (if (Math|Float|InRange(Float) (Variables|AutoSPVariables|GetCurrentFps) (- _desiredframerate 5.0) (+ _desiredframerate 3.0))
          (Utilities|FlowControl|Gate false :!label _label
            (:Exit
              (Variables|HMDSettings|SetCurrentSP (+ (Variables|HMDSettings|GetCurrentSP) 5.0))
              (Development|ExecuteConsoleCommand (Utilities|String|Append "hmd sp " (Utilities|String|ToString(Float) (Variables|HMDSettings|GetCurrentSP))))))
          (else
            (Utilities|FlowControl|Sequence
              (:then_0
                (Utilities|FlowControl|Gate true :!label _label_2
                  (:Exit
                    (Variables|HMDSettings|SetCurrentSP (- (Variables|HMDSettings|GetCurrentSP) 6.0))
                    (Development|ExecuteConsoleCommand (Utilities|String|Append "hmd sp " (Utilities|String|ToString(Float) (Variables|HMDSettings|GetCurrentSP))))
                    (Utilities|FlowControl|Sequence
                      (:then_0
                        (goto _label Close))
                      (:then_1
                        (Utilities|FlowControl|RetriggerableDelay 15.0)
                        (goto _label Open))))))
              (:then_1
                (if (< (Variables|AutoSPVariables|GetCurrentFps) (- (Variables|AutoSPVariables|GetDesiredFrameRate) 7.0))
                  (goto _label_2 Open)
                  (else
                    (goto _label_2 Close)))))))))
    (:then_1
      ;[1 1 1] Highlight Scene Componens, Toggle and animate based on time
      (if (Variables|HighlightingAndInteraction|GetPlayerCanInteractWithTrace)
        (Utilities|FlowControl|Sequence
          (:then_0
            (bind (_hitinteractiveobject _component) (CallFunction|CheckforInteractiveObjects))
            (if _hitinteractiveobject
              (CallFunction|HighlightInteractiveObject _component)
              (elif (Variables|HighlightingAndInteraction|GetDoesHighlightStick)
                (Variables|HighlightingAndInteraction|SetIsUpdateingTimeBaseMaterial false)
                (elif (!= (Variables|HighlightingAndInteraction|GetHighlightedObject) (Variables|HighlightingAndInteraction|GetLookingAtComponent))
                  (for _array_element (Components|GetChildrenComponents (Variables|HighlightingAndInteraction|GetHighlightedObject) true)
                    (if (Components|ComponentHasTag _array_element "CanHighlight")
                      (bind _asprimitivecomponent (Utilities|Casting|CastToPrimitiveComponent _array_element))
                      (bind _returnvalue_4 (Rendering|Material|CreateDynamicMaterialInstance _asprimitivecomponent 0 0 :!class /Script/Engine.PrimitiveComponent))
                      (Rendering|Material|SetScalarParameterValue _returnvalue_4 "HighlightedAmount" 0.0 :!class /Script/Engine.MaterialInstanceDynamic)
                      (elif (Components|ComponentHasTag _array_element "ToggleOnView")
                        (Rendering|SetVisibility _array_element false false))))
                  (Variables|HighlightingAndInteraction|SetHighlightedAmount 0)
                  (Variables|HighlightingAndInteraction|SetIsUpdateingTimeBaseMaterial false)))))
          (:then_1
            (if (Variables|HighlightingAndInteraction|GetIsUpdateingTimeBaseMaterial)
              (bind _asprimitivecomponent_2 (Utilities|Casting|CastToPrimitiveComponent _highlightedtimechangingobject))
              (bind _returnvalue_5 (Rendering|Material|CreateDynamicMaterialInstance _asprimitivecomponent_2 0 0 :!class /Script/Engine.PrimitiveComponent))
              (Rendering|Material|SetScalarParameterValue _returnvalue_5 "SecondsLookedAt" (Variables|HighlightingAndInteraction|GetAmountOfTimeLookedAtObject) :!class /Script/Engine.MaterialInstanceDynamic)
              (else
                (bind _asprimitivecomponent_3 (Utilities|Casting|CastToPrimitiveComponent _highlightedtimechangingobject))
                (bind _returnvalue_6 (Rendering|Material|CreateDynamicMaterialInstance _asprimitivecomponent_3 0 0 :!class /Script/Engine.PrimitiveComponent))
                (Variables|HighlightingAndInteraction|SetAmountOfTimeLookedAtObject (Math|Interpolation|FInterpTo (Variables|HighlightingAndInteraction|GetAmountOfTimeLookedAtObject) 0.0 (Variables|AutoSPVariables|GetDeltaSeconds) 2.0))
                (Rendering|Material|SetScalarParameterValue _returnvalue_6 "SecondsLookedAt" (Variables|HighlightingAndInteraction|GetAmountOfTimeLookedAtObject) :!class /Script/Engine.MaterialInstanceDynamic)))))))
    (:then_2
      ;[1 1 1] Rotate Towards HMD
      (if (and (Variables|RotatePawnTowardsHMDOrientation|GetDoesRotateTowardsHMDOrientation) (Class|HeadMountedDisplayFunctionLibrary|IsHeadMountedDisplayEnabled))
        (if (Variables|RotatePawnTowardsHMDOrientation|GetTankModeWhileNotMoving)
          (bind _ascharacter (Utilities|Casting|CastToCharacter (Pawn|GetControlledPawn)))
          (if (not (== (Transformation|GetVelocity _ascharacter) "0, 0, 0"))
            (if (Variables|RotatePawnTowardsHMDOrientation|GetRotateCameraAndBody) :!label _label_3
              ;;[1 1 1] Rotate Camera And Body
              (if (not (Math|Float|InRange(Float) _yaw_2 (* _pawnrotationanglekeyhole -1.0) _pawnrotationanglekeyhole))
                (Pawn|SetControlRotation (Class|KismetMathLibrary|MakeRot _pitch (+ _yaw (* (Math|Float|Sign(Float) _yaw_2) (Variables|RotatePawnTowardsHMDOrientation|GetRotateTowardsHMDSpeed))) _roll)))
              (else
                ;;[1 1 1] Rotate Just Camera
                (bind _ascharacter_2 (Utilities|Casting|CastToCharacter (Pawn|GetControlledPawn)))
                (Transformation|SetWorldRotation (Variables|/Script/Engine.Character|GetMesh _ascharacter_2) (Math|Interpolation|RInterpTo (Transformation|GetWorldRotation (Variables|/Script/Engine.Character|GetMesh _ascharacter_2)) (Class|KismetMathLibrary|MakeRot (.Pitch (Class|KismetMathLibrary|BreakRot (Transformation|GetWorldRotation (Variables|/Script/Engine.Character|GetMesh _ascharacter_2)))) (.Yaw (Class|KismetMathLibrary|BreakRot (Math|Rotator|CombineRotators (Math|Rotator|FindLookatRotation _returnvalue_3 (+ _returnvalue_3 (* (Transformation|GetActorForwardVector _returnvalue_2) (Variables|HighlightingAndInteraction|GetInteractionDistance)))) "0,-90.000000, 0"))) (.Roll (Class|KismetMathLibrary|BreakRot (Transformation|GetWorldRotation (Variables|/Script/Engine.Character|GetMesh _ascharacter_2))))) (Utilities|Time|GetWorldDeltaSeconds) (Variables|RotatePawnTowardsHMDOrientation|GetRotateTowardsHMDSpeed)) false))))
          (else
            (goto _label_3)))))
    (:then_3
      ;[1 1 1] If we walk away from menu turn off
      (if (Variables|Default|GetIsMenuOpen)
        (if (> (Math|Vector|VectorLength (- (Transformation|GetActorLocation (Game|GetPlayerCharacter 0)) (Transformation|GetActorLocation (Variables|Default|GetCurrentlyOpenMenu)))) 2e+02)
          (CallFunction|ToggleMenu))))))

(event Input|ActionEvents|InputActionFire
  (bind _returnvalue (Game|GetPlayerCameraManager 0))
  (bind _returnvalue_2 (Transformation|GetActorLocation _returnvalue))
  (bind _returnvalue_3 (Transformation|GetActorRotation _returnvalue))
  (bind _returnvalue_4 (Transformation|GetActorForwardVector _returnvalue))
  (bind _returnvalue_5 (* _returnvalue_4 5e+01))
  (bind _returnvalue_6 (+ _returnvalue_5 _returnvalue_2))
  ;[1 1 1] Shoot grappling hook
  (:Pressed
    (if (Class|HeadMountedDisplayFunctionLibrary|IsHeadMountedDisplayEnabled)
      (bind _returnvalue_7 (Game|SpawnActorfromClass "/Game/Blueprints/GrapplingHook.GrapplingHook_C" (Math|Transform|MakeTransform (+ _returnvalue_5 (+ _returnvalue_2 "0,0.000000,0.000000")) _returnvalue_3 "1,1.000000,1") true))
      (Variables|Default|SetLast%20GrapplingHook _returnvalue_7)
      (else
        (bind _returnvalue_8 (Game|SpawnActorfromClass "/Game/Blueprints/GrapplingHook.GrapplingHook_C" (Math|Transform|MakeTransform _returnvalue_6 _returnvalue_3 "1.000000,1.000000,1") true))
        (Variables|Default|SetLast%20GrapplingHook _returnvalue_8)))
    (Audio|PlaySoundatLocation "/Game/Audio/fire_grapplinghook_Cue.fire_grapplinghook_Cue" _returnvalue_6))
  (:Released
    (Actor|DestroyActor (Variables|Default|GetLast%20GrapplingHook))
    (Variables|/Script/Engine.CharacterMovementComponent|SetGravityScale (Variables|/Script/Engine.Character|GetCharacterMovement (Game|GetPlayerCharacter 0)) 1.0)))

(event Input|ActionEvents|InputActionOpenMenu
  ;[1 1 1] Menu
  (:Pressed
    (CallFunction|ToggleMenu)))

(event Input|GamepadEvents|GamepadRightTrigger
  (bind _returnvalue (Game|GetPlayerCameraManager 0))
  (bind _returnvalue_2 (Transformation|GetActorLocation _returnvalue))
  (bind _returnvalue_3 (Transformation|GetActorRotation _returnvalue))
  (bind _returnvalue_4 (Transformation|GetActorForwardVector _returnvalue))
  (bind _returnvalue_5 (* _returnvalue_4 5e+01))
  (bind _returnvalue_6 (+ _returnvalue_5 _returnvalue_2))
  ;[1 1 1] Shoot grappling hook
  (:Pressed
    (if (Class|HeadMountedDisplayFunctionLibrary|IsHeadMountedDisplayEnabled)
      (bind _returnvalue_7 (Game|SpawnActorfromClass "/Game/Blueprints/GrapplingHook.GrapplingHook_C" (Math|Transform|MakeTransform (+ _returnvalue_5 (+ _returnvalue_2 "0,0.000000,0.000000")) _returnvalue_3 "1,1.000000,1") true))
      (Variables|Default|SetLast%20GrapplingHook _returnvalue_7)
      (else
        (bind _returnvalue_8 (Game|SpawnActorfromClass "/Game/Blueprints/GrapplingHook.GrapplingHook_C" (Math|Transform|MakeTransform _returnvalue_6 _returnvalue_3 "1.000000,1.000000,1") true))
        (Variables|Default|SetLast%20GrapplingHook _returnvalue_8)))
    (Audio|PlaySoundatLocation "/Game/Audio/fire_grapplinghook_Cue.fire_grapplinghook_Cue" _returnvalue_6))
  (:Released
    (Actor|DestroyActor (Variables|Default|GetLast%20GrapplingHook))
    (Variables|/Script/Engine.CharacterMovementComponent|SetGravityScale (Variables|/Script/Engine.Character|GetCharacterMovement (Game|GetPlayerCharacter 0)) 1.0)))

(event Input|KeyboardEvents|Escape
  ;[1 1 1] Exit and save
  (:Pressed
    (if (Variables|Default|GetIsMenuOpen)
      (CallFunction|ToggleMenu)
      (else
        (CallFunction|SaveHMDSettings)
        (Game|QuitGame)))))

(event Input|KeyboardEvents|CtrlR
  (:Pressed
    (Development|ExecuteConsoleCommand "stereo on")))

(event Input|KeyboardEvents|ShiftR
  ;[1 1 1] Reset HMD
  (:Pressed
    (Class|HeadMountedDisplayFunctionLibrary|ResetOrientationandPosition 0.0)))

(event Input|KeyboardEvents|CtrlT
  (:Pressed
    (Development|ExecuteConsoleCommand "sg.ViewDistanceQuality 0")
    (Development|ExecuteConsoleCommand "sg.PostProcessQuality 0")
    (Development|ExecuteConsoleCommand "sg.AntiAliasingQuality 0")
    (Development|ExecuteConsoleCommand "sg.ShadowQuality 1")
    (Development|ExecuteConsoleCommand "sg.TextureQuality 1")
    (Development|ExecuteConsoleCommand "sg.EffectsQuality 0")
    (Development|ExecuteConsoleCommand "hmd vsync off")))

(fn ConstructionScript)

(fn ManuallyChangeScreenPercentage
  (Variables|HMDSettings|SetCurrentSP (Math|Float|Clamp(Float) (Variables|HMDSettings|GetCurrentSP) (Variables|HMDSettings|GetLowestSP) (Variables|HMDSettings|GetHighestSP)))
  (Development|ExecuteConsoleCommand (Utilities|String|Append "hmd sp " (Utilities|String|ToString(Float) (Variables|HMDSettings|GetCurrentSP)))))

(fn ManuallyChangeDistortionScale
  (Variables|HMDSettings|SetCurrentDistortionScale (Math|Float|Clamp(Float) (Variables|HMDSettings|GetCurrentDistortionScale) 0.2 2.0))
  (Development|ExecuteConsoleCommand (Utilities|String|Append (Utilities|String|Append (Utilities|String|Append "oculusdev on | " "hmdwarp 1=1 | ") "hmdwarp s=") (Utilities|String|ToString(Float) (Variables|HMDSettings|GetCurrentDistortionScale)))))

(fn CheckforInteractiveObjects
  (bind _returnvalue (Game|GetPlayerCameraManager 0))
  (bind _returnvalue_2 (Transformation|GetActorForwardVector _returnvalue))
  (bind _returnvalue_3 (Transformation|GetActorLocation _returnvalue))
  (bind (_outhit _returnvalue_4) (Collision|LineTraceForObjects _returnvalue_3 (+ _returnvalue_3 (* _returnvalue_2 (Variables|HighlightingAndInteraction|GetInteractionDistance))) (Utilities|Array|MakeArray "ObjectTypeQuery2" "ObjectTypeQuery1" "ObjectTypeQuery4") false (Utilities|Array|MakeArray (Game|Player|GetPlayerPawn 0)) "None"))
  (if _returnvalue_4
    (Variables|Default|SetImpactPoint (.ImpactPoint (Collision|BreakHitResult _outhit)))
    (Variables|HighlightingAndInteraction|SetLookingAtComponent (.HitComponent (Collision|BreakHitResult _outhit)))
    (return (Components|ComponentHasTag (.HitComponent (Collision|BreakHitResult _outhit)) "Interactive") (.HitComponent (Collision|BreakHitResult _outhit)) (.HitActor (Collision|BreakHitResult _outhit)))
    (else
      (Variables|Default|SetImpactPoint (+ _returnvalue_3 (* _returnvalue_2 1e+03))))))

(fn HighlightInteractiveObject
  (params (LookingAtObject :type Primitive%20Component%20Object%20Reference))
  (if (== (Variables|HighlightingAndInteraction|GetHighlightedAmount) 0)
    (for _array_element (Components|GetChildrenComponents LookingAtObject true)
      (if (Components|ComponentHasTag _array_element "CanHighlight")
        (bind _asprimitivecomponent (Utilities|Casting|CastToPrimitiveComponent _array_element))
        (bind _returnvalue (Rendering|Material|CreateDynamicMaterialInstance _asprimitivecomponent 0 0 :!class /Script/Engine.PrimitiveComponent))
        (Rendering|Material|SetScalarParameterValue _returnvalue "HighlightedAmount" 1.0 :!class /Script/Engine.MaterialInstanceDynamic)
        (if (Components|ComponentHasTag _array_element "EffectedByTime")
          (Variables|HighlightingAndInteraction|SetHighlightedTimeChangingObject _array_element))
        (elif (Components|ComponentHasTag _array_element "ToggleOnView")
          (Rendering|SetVisibility _array_element true false))))
    (Variables|HighlightingAndInteraction|SetHighlightedObject LookingAtObject)
    (Variables|HighlightingAndInteraction|SetHighlightedAmount 1)
    (elif (Variables|HighlightingAndInteraction|GetDoesHighlightStick)
      (if (!= LookingAtObject (Variables|HighlightingAndInteraction|GetHighlightedObject))
        (for _array_element_2 (Components|GetChildrenComponents (Variables|HighlightingAndInteraction|GetHighlightedObject) true)
          (if (Components|ComponentHasTag _array_element_2 "CanHighlight")
            (bind _asprimitivecomponent_2 (Utilities|Casting|CastToPrimitiveComponent _array_element_2))
            (bind _returnvalue_2 (Rendering|Material|CreateDynamicMaterialInstance _asprimitivecomponent_2 0 0 :!class /Script/Engine.PrimitiveComponent))
            (Rendering|Material|SetScalarParameterValue _returnvalue_2 "HighlightedAmount" 0.0 :!class /Script/Engine.MaterialInstanceDynamic)
            (elif (Components|ComponentHasTag _array_element_2 "ToggleOnView")
              (Rendering|SetVisibility _array_element_2 false false))))
        (Variables|HighlightingAndInteraction|SetHighlightedAmount 0)
        (Variables|HighlightingAndInteraction|SetIsUpdateingTimeBaseMaterial false)
        (else
          (Variables|HighlightingAndInteraction|SetAmountOfTimeLookedAtObject (+ (Variables|HighlightingAndInteraction|GetAmountOfTimeLookedAtObject) (Variables|AutoSPVariables|GetDeltaSeconds)) :!label _label)
          (Variables|HighlightingAndInteraction|SetIsUpdateingTimeBaseMaterial true)))
      (else
        (goto _label)))))

(fn SaveHMDSettings
  (bind _ashmdsettingssave_c (Utilities|Casting|CastToHMDSettingsSave (Variables|Default|GetHMDSettingsSave)))
  (Variables|/Game/Blueprints/HMDSettingsSave.HMDSettingsSave_C|SetCurrentSP _ashmdsettingssave_c (Variables|HMDSettings|GetCurrentSP))
  (Variables|/Game/Blueprints/HMDSettingsSave.HMDSettingsSave_C|SetHighestSP _ashmdsettingssave_c (Variables|HMDSettings|GetHighestSP))
  (Variables|/Game/Blueprints/HMDSettingsSave.HMDSettingsSave_C|SetLowestSP _ashmdsettingssave_c (Variables|HMDSettings|GetLowestSP))
  (Variables|/Game/Blueprints/HMDSettingsSave.HMDSettingsSave_C|SetDistortionScale _ashmdsettingssave_c (Variables|HMDSettings|GetCurrentDistortionScale))
  (SaveGame|SaveGametoSlot (Variables|Default|GetHMDSettingsSave) "HMDSettings"))

(fn ToggleMenu
  (bind _returnvalue (Game|GetPlayerCameraManager 0))
  (bind _returnvalue_2 (Transformation|GetActorTransform _returnvalue))
  (bind _returnvalue_3 (Transformation|GetActorForwardVector _returnvalue))
  (bind (_location _rotation _scale) (Math|Transform|BreakTransform _returnvalue_2))
  (if (Variables|Default|GetIsMenuOpen)
    (Actor|DestroyActor (Variables|Default|GetCurrentlyOpenMenu))
    (Variables|Default|SetIsMenuOpen false)
    (Variables|HighlightingAndInteraction|SetDoesHighlightStick (Variables|Default|GetBeforeMenuHighlighting))
    (else
      (Variables|Default|SetBeforeMenuHighlighting (Variables|HighlightingAndInteraction|GetDoesHighlightStick))
      (bind _returnvalue_4 (Game|SpawnActorfromClass "/Game/Blueprints/ContextMenu.ContextMenu_C" (Math|Transform|MakeTransform (+ _location (* _returnvalue_3 1e+02)) (Math|Rotator|MakeRotfromXZ (* _returnvalue_3 -1.0) (Transformation|GetActorUpVector (Game|GetPlayerCharacter 0))) _scale) true))
      (Variables|Default|SetCurrentlyOpenMenu _returnvalue_4)
      (Variables|Default|SetIsMenuOpen true)
      (Variables|HighlightingAndInteraction|SetDoesHighlightStick true))))

(fn ManuallyChangeIPD
  (if (Variables|Default|GetIPDOverride)
    (Development|ExecuteConsoleCommand (Utilities|String|Append "stereo e=" (Utilities|String|ToString(Float) (/ (Variables|HMDSettings|GetCurrentIPD) 1e+03))))
    (else
      (Development|ExecuteConsoleCommand "stereo reset"))))

(fn ManuallyChangeVsync
  (if (Variables|Default|GetVsyncEnabled)
    (Development|ExecuteConsoleCommand "hmd vsync on")
    (else
      (Development|ExecuteConsoleCommand "hmd vsync Off"))))

(fn ManuallyChangeScalabilitySettings
  (Development|ExecuteConsoleCommand (Utilities|String|Append "sg.PostProcessQuality " (Utilities|String|ToString(Float) (Variables|ScalabilitySettings|GetCurrentPostProcessQuality))))
  (Development|ExecuteConsoleCommand (Utilities|String|Append "sg.ShadowQuality " (Utilities|String|ToString(Float) (Variables|ScalabilitySettings|GetCurrentShadowQuality))))
  (Development|ExecuteConsoleCommand (Utilities|String|Append "sg.TextureQuality " (Utilities|String|ToString(Float) (Variables|ScalabilitySettings|GetCurrentTextureQuality))))
  (Development|ExecuteConsoleCommand (Utilities|String|Append "sg.EffectsQuality " (Utilities|String|ToString(Float) (Variables|ScalabilitySettings|GetCurrentEffectsQuality))))
  (Development|ExecuteConsoleCommand (Utilities|String|Append "r.ViewDistanceScale " (Utilities|String|ToString(Float) (Math|Float|Clamp(Float) (Variables|ScalabilitySettings|GetCurrentViewDistanceScale) 0.1 2.0))))
  (Development|ExecuteConsoleCommand (Utilities|String|Append "r.PostProcessAAQuality " (Utilities|String|ToString(Float) (Math|Float|Clamp(Float) (Variables|ScalabilitySettings|GetCurrentAAQuality) 0.0 6.0)))))