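; Grappling hook projectile that pulls the player to grappable surfaces or drags pullable actors toward the player, trailing a cable from the camera.
; On impact it attaches and reads the hit material instance's first scalar parameter to choose the behavior, otherwise it destroys itself.
; Tick launches the player or moves the target; reaching the hook zeroes gravity and pins the player there.
; A flight timer zeroes the projectile's velocity.
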(event OnProjectileStop(ProjectileMovement1)
  (params (ImpactResult :type Hit%20Result%20Structure%20%28by%20ref%29))
  (bind (_location _normal _impactpoint _impactnormal _physmat _hitactor _hitcomponent) (Collision|BreakHitResult ImpactResult))
  ;[1 1 1] Hook hits object
  (Utilities|FlowControl|Sequence
    (:then_0
      (Variables|Default|SetLast%20Hit%20Actor _hitactor))
    (:then_1
      (Class|Actor|AttachRootComponenttoActor _hitactor "None" "KeepWorldPosition"))
    (:then_2
      (bind _asmaterialinstanceconstant (Utilities|Casting|CastToMaterialInstanceConstant (Rendering|Material|GetMaterial _hitcomponent 0))
        (:then
          ;[1 1 1] Determine grappling behaviour
          (if (and (Utilities|Name|Equal(Name) (.ParameterName (Utilities|Struct|BreakScalarParameterValue (Utilities|Array|Get(acopy) (Variables|/Script/Engine.MaterialInstance|GetScalarParameterValues _asmaterialinstanceconstant)))) "Pullable") (== (.ParameterValue (Utilities|Struct|BreakScalarParameterValue (Utilities|Array|Get(acopy) (Variables|/Script/Engine.MaterialInstance|GetScalarParameterValues _asmaterialinstanceconstant)))) 1.0))
            (Variables|Default|SetPull%20Pullable%20In true)
            (Audio|PlaySoundatLocation "/Game/Audio/HookImpact_Cue.HookImpact_Cue" _location :!label _label)
            (elif (and (Utilities|Name|Equal(Name) (.ParameterName (Utilities|Struct|BreakScalarParameterValue (Utilities|Array|Get(acopy) (Variables|/Script/Engine.MaterialInstance|GetScalarParameterValues _asmaterialinstanceconstant)))) "Grappable") (== (.ParameterValue (Utilities|Struct|BreakScalarParameterValue (Utilities|Array|Get(acopy) (Variables|/Script/Engine.MaterialInstance|GetScalarParameterValues _asmaterialinstanceconstant)))) 1.0))
              (Variables|Default|SetPullPlayerIn true)
              (goto _label)
              (else
                (Audio|PlaySoundatLocation "/Game/Audio/HookRecoil_Cue.HookRecoil_Cue" _location :!label _label_2)
                (Actor|DestroyActor)))))
        (:CastFailed
          (goto _label_2))))))

(event EventTick
  (params (DeltaSeconds :type Float%20%28single-precision%29))
  (bind _returnvalue (Transformation|GetActorLocation))
  (bind _returnvalue_2 (Game|GetPlayerCameraManager 0))
  (bind _returnvalue_3 (Game|GetPlayerCharacter 0))
  (bind _launch_force_per_second (Variables|Default|GetLaunch%20Force%20per%20Second))
  (bind _last_hit_actor (Variables|Default|GetLast%20Hit%20Actor))
  (bind _returnvalue_4 (Transformation|GetActorLocation _last_hit_actor))
  (bind _returnvalue_5 (Transformation|GetActorLocation _returnvalue_2))
  (bind _returnvalue_6 (Math|Rotator|FindLookatRotation _returnvalue_5 _returnvalue))
  (bind _returnvalue_7 (Math|Vector|GetForwardVector _returnvalue_6))
  (bind _returnvalue_8 (* _returnvalue_7 _launch_force_per_second))
  (Utilities|FlowControl|Sequence
    (:then_0
      (if (Variables|Default|GetPullPlayerIn)
        ;[1 1 1] Launch player towards hook
        (Character|LaunchCharacter _returnvalue_3 (* (+ _returnvalue_8 (* (- _returnvalue_8 (Transformation|GetVelocity _returnvalue_3)) 1.0)) DeltaSeconds) false false)
        (else
          ;[1 1 1] Keep the player in place
          (if (Variables|Default|GetFreeze%20Player)
            (Variables|/Script/Engine.MovementComponent|SetVelocity (Pawn|GetMovementComponent _returnvalue_3) "0, 0,0.000000")
            (Transformation|SetActorLocation _returnvalue_3 (+ (Transformation|GetActorLocation) (Variables|Default|GetRelative%20Freeze%20Location)) false)
            (else
              ;[1 1 1] Pull pullable
              (if (Variables|Default|GetPull%20Pullable%20In)
                (if (== (Utilities|Array|Length (Class|SceneComponent|GetParentComponents (VehicleSound|GetRootComponent))) 0)
                  (Actor|DestroyActor)
                  (else
                    (Transformation|SetActorLocation _last_hit_actor (+ _returnvalue_4 (* (Class|KismetMathLibrary|GetDirectionVector _returnvalue_4 (Transformation|GetActorLocation (Game|GetPlayerCharacter 0))) (* DeltaSeconds 5e+02))) false)))))))))
    (:then_1
      ;[1 1 1] Keep cable connected to the player
      (Transformation|SetWorldLocation (Variables|Default|GetCable1) (+ _returnvalue_5 "0, 0,-30.000000") false))))

(event EventBeginPlay
  (Utilities|Time|SetTimerbyFunctionName 0 "FlightTimeEnd" (Variables|Default|GetFlight%20Time)))

(event EventHit
  (params (MyComp :type Primitive%20Component%20Object%20Reference) (Other :type Actor%20Object%20Reference) (OtherComp :type Primitive%20Component%20Object%20Reference) (bSelfMoved :type Boolean) (HitLocation :type Vector :default "0, 0, 0") (HitNormal :type Vector :default "0, 0, 0") (NormalImpulse :type Vector :default "0, 0, 0") (Hit :type Hit%20Result%20Structure%20%28by%20ref%29))
  (bind _returnvalue (Game|GetPlayerCharacter 0))
  ;[1 1 1] Freeze player when he reaches the hook
  (if (== Other _returnvalue)
    (if (Variables|Default|GetPullPlayerIn)
      (Variables|Default|SetPullPlayerIn false)
      (Variables|Default|SetPull%20Pullable%20In false)
      (Variables|/Script/Engine.CharacterMovementComponent|SetGravityScale (Variables|/Script/Engine.Character|GetCharacterMovement _returnvalue) 0.0)
      (Variables|Default|SetFreeze%20Player true)
      (Variables|Default|SetRelative%20Freeze%20Location (- (Transformation|GetActorLocation _returnvalue) (Transformation|GetActorLocation))))))

(fn ConstructionScript)

(fn FlightTimeEnd
  (Variables|/Script/Engine.MovementComponent|SetVelocity (Variables|Default|GetProjectileMovement1) "0, 0, 0"))