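; A world text counter that shows the player's collected coins against a target number.
; Each tick it reads CoinCount from the MyCharacterExplorationNoHeadBob player character and displays it as "count/target" on CoinCounterText.
; The first time the count reaches CoinTargetNumber, a DoOnce turns the text green and calls AllCoinsCollected with the target number.
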(event EventTick
  (params (DeltaSeconds :type Float%20%28single-precision%29))
  (bind _cointargetnumber (Variables|Default|GetCoinTargetNumber))
  (bind _coincounter_text (Variables|Default|GetCoinCounter_Text))
  (bind _asmycharacterexplorationnoheadbob_c (Utilities|Casting|CastToMyCharacterExplorationNoHeadBob (Game|GetPlayerCharacter 0)))
  (Rendering|Components|TextRender|SetText _coincounter_text (Utilities|String|Append (Utilities|String|Append (Utilities|String|ToString(Integer) (Variables|/Game/Blueprints/MyCharacterExplorationNoHeadBob.MyCharacterExplorationNoHeadBob_C|GetCoin%20Count _asmycharacterexplorationnoheadbob_c)) " / ") (Utilities|String|ToString(Integer) _cointargetnumber)))
  (if (not (< (Variables|/Game/Blueprints/MyCharacterExplorationNoHeadBob.MyCharacterExplorationNoHeadBob_C|GetCoin%20Count _asmycharacterexplorationnoheadbob_c) _cointargetnumber))
    (Utilities|FlowControl|DoOnce false
      (:Completed
        (Rendering|Components|TextRender|SetTextRenderColor _coincounter_text (Math|Color|MakeColor 0 255 0 255))
        (Default|CallAllCoinsCollected _cointargetnumber)))))

(fn ConstructionScript)